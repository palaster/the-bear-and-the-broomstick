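; Forest golem enemy Blueprint that idles, wanders the navmesh, and runs at the player once perception detects them.
; An AIState enum, switched in UpdateAIState, drives movement events, with AIMoveTo results choosing the next state.
; In Attack it stops moving, and weapon overlaps damage each actor once, tracked in a list cleared on entering Attack.
; Damage reduces HP until a death animation and destroy; the flinch-on-hit reaction is unwired.
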(event OnTargetPerceptionUpdated(AIPerception)
  (params (Actor :type Actor%20Object%20Reference) (Stimulus :type AI%20Stimulus%20Structure))
  (if (== (Utilities|GetClass Actor) "/Game/Player/Player.Player_C")
    (Variables|Default|SetEnemy Actor)
    (CallFunction|UpdateAIState "NewEnumerator3")))

(event OnComponentBeginOverlap(Weapon)
  (params (OverlappedComponent :type Primitive%20Component%20Object%20Reference) (OtherActor :type Actor%20Object%20Reference) (OtherComp :type Primitive%20Component%20Object%20Reference) (OtherBodyIndex :type Integer) (bFromSweep :type Boolean) (SweepResult :type Hit%20Result%20Structure%20%28by%20ref%29))
  (if (|Candealdamage OtherActor)
    (if (not (Utilities|Set|Contains (Variables|Default|GetDamagedActors) OtherActor))
      (Utilities|Set|Add (Variables|Default|GetDamagedActors) OtherActor)
      (Game|Damage|ApplyDamage OtherActor (Variables|Default|GetTrunkDamage) (Pawn|GetController) self "/Engine/EngineDamageTypes/DmgTypeBP_Environmental.DmgTypeBP_Environmental_C"))))

(event Custom|OnTakeAnyDamage_Event_0
  (params (DamagedActor :type Actor%20Object%20Reference) (Damage :type Float%20%28single-precision%29) (DamageType :type Damage%20Type%20Object%20Reference) (InstigatedBy :type Controller%20Object%20Reference) (DamageCauser :type Actor%20Object%20Reference))
  (bind _output_get (Variables|Default|SetHP (- (Variables|Default|GetHP) Damage)))
  (if (<= _output_get 0.0)
    (Variables|/Script/Engine.CharacterMovementComponent|SetMaxWalkSpeed (Variables|Character|GetCharacterMovement) 0.0)
    (Components|Animation|PlayAnimation (Variables|Character|GetMesh) "/Game/Creatures/ForestGolems/Animations/Common/G_C_Die1.G_C_Die1" false)
    (Utilities|FlowControl|Delay 3.0)
    (Actor|DestroyActor)))

(event Custom|Wander_Event
  (bind _movementresult (AI|AIMoveTo (Variables|Default|GetNav%20Mesh) self (.RandomLocation (AI|Navigation|GetRandomReachablePointinRadius (Transformation|GetActorLocation) 1e+03 (Variables|Default|GetNav%20Mesh) 0)) 0 5e+01 true)
    (:OnSuccess
      (CallFunction|UpdateAIState "NewEnumerator0"))
    (:OnFail
      (if (not (Utilities|Enum|Equal(Enum) _movementresult "Aborted"))
        (CallFunction|UpdateAIState "NewEnumerator1")))))

(event Custom|AttackMove_Event
  (bind _movementresult (AI|AIMoveTo (Variables|Default|GetNav%20Mesh) self "0, 0, 0" (Variables|Default|GetEnemy) 5e+01 true)
    (:OnSuccess
      (CallFunction|UpdateAIState "NewEnumerator4"))
    (:OnFail
      (switch Utilities|FlowControl|Switch|SwitchonEPathFollowingResult _movementresult
        (:Blocked
          _)
        (:OffPath
          _)
        (:Aborted
          _)
        (:Invalid
          _))
      (CallFunction|UpdateAIState "NewEnumerator0"))))

(event Custom|Attack_Event
  (Pawn|Components|CharacterMovement|DisableMovement (Variables|Character|GetCharacterMovement)))

(event Custom|Idle_Event
  (Variables|Default|SetTimeIdled 0.0)
  (Variables|Default|SetIdleTime (Math|Conversions|ToFloat(Integer) (* (Math|Random|RandomInteger 3) 2)))
  (Components|Movement|StopMovementImmediately (Variables|Character|GetCharacterMovement)))

(event Custom|Flee_Event
  (Variables|Default|SetFlinch true)
  (Variables|/Script/Engine.CharacterMovementComponent|SetMaxWalkSpeed (Variables|Character|GetCharacterMovement) (Variables|Default|GetRun%20Speed))
  (Utilities|Time|SetTimerbyFunctionName 0 "Reset Walk Speed" 15.0))

(event EventBeginPlay
  (EventDispatchers|AssignOnTakeAnyDamage (delegate Custom|OnTakeAnyDamage_Event_0))
  (bind _outactors (Actor|GetAllActorsOfClass "/Script/NavigationSystem.NavigationData"))
  (for _array_element _outactors
    (Variables|Default|SetNav%20Mesh _array_element))
  (CallFunction|UpdateAIState "NewEnumerator0"))

(event EventTick
  (params (DeltaSeconds :type Float%20%28single-precision%29))
  (if (Utilities|Enum|Equal(Enum) (Variables|Default|GetAI%20State) "NewEnumerator0")
    (bind _output_get (Variables|Default|SetTimeIdled (+ (Variables|Default|GetTimeIdled) DeltaSeconds)))
    (if (>= _output_get (Variables|Default|GetIdleTime))
      (CallFunction|UpdateAIState "NewEnumerator1"))))

(fn ConstructionScript
  (CallFunction|ResetWalkSpeed))

(fn ResetWalkSpeed
  (Variables|/Script/Engine.CharacterMovementComponent|SetMaxWalkSpeed (Variables|Character|GetCharacterMovement) (Variables|Default|GetWalk%20Speed)))

(fn UpdateAIState
  (params (NewParam :type AI_Combat_State%20Enum :default "NewEnumerator0"))
  (bind _output_get (Variables|Default|SetAI%20State NewParam))
  (switch Utilities|FlowControl|Switch|SwitchonAI_Combat_State _output_get
    (:NewEnumerator0
      (CallFunction|IdleEvent))
    (:NewEnumerator1
      (CallFunction|ResetWalkSpeed)
      (CallFunction|WanderEvent))
    (:NewEnumerator5
      (Pawn|Components|CharacterMovement|DisableMovement (Variables|Character|GetCharacterMovement)))
    (:NewEnumerator3
      (Variables|/Script/Engine.CharacterMovementComponent|SetMaxWalkSpeed (Variables|Character|GetCharacterMovement) (Variables|Default|GetRun%20Speed))
      (CallFunction|AttackMoveEvent))
    (:NewEnumerator4
      (Utilities|Set|Clear (Variables|Default|GetDamagedActors))
      (CallFunction|AttackEvent))))

(fn Unflinch
  (Pawn|Components|CharacterMovement|SetMovementMode (Variables|Character|GetCharacterMovement) "MOVE_Walking" 0)
  (CallFunction|UpdateAIState "NewEnumerator3"))