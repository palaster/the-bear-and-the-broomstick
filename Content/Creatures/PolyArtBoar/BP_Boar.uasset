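; Boar creature that endlessly wanders to random reachable navmesh points, pausing for a random time between moves when at walk speed.
; Construction randomizes its body mesh, fur material and tusk mesh for variety.
; Damage reduces HP, sets a flinch flag, disables movement and raises max speed until a timer resets it.
; At zero HP it plays a death animation, then destroys itself after a delay.
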(event Custom|Wander_Event
  (bind _output_get (Variables|Default|SetWaypoint (.RandomLocation (AI|Navigation|GetRandomReachablePointinRadius (Transformation|GetActorLocation) 1e+03 (Variables|Default|GetNav%20Mesh) 0))))
  (AI|AIMoveTo (Variables|Default|GetNav%20Mesh) self _output_get 0 5e+01 true
    (:OnSuccess
      (if (> (Variables|/Script/Engine.CharacterMovementComponent|GetMaxWalkSpeed (Variables|Character|GetCharacterMovement)) 1e+02)
        _
        (else
          (Utilities|FlowControl|Delay (Math|Conversions|ToFloat(Integer) (* (Math|Random|RandomInteger 3) 2))))))
    (:OnFail
      _))
  (CallFunction|WanderEvent))

(event Custom|OnTakeAnyDamage_Event_0
  (params (DamagedActor :type Actor%20Object%20Reference) (Damage :type Float%20%28single-precision%29) (DamageType :type Damage%20Type%20Object%20Reference) (InstigatedBy :type Controller%20Object%20Reference) (DamageCauser :type Actor%20Object%20Reference))
  (bind _output_get (Variables|Default|SetHP (- (Variables|Default|GetHP) Damage)))
  (if (<= _output_get 0.0)
    (Variables|/Script/Engine.CharacterMovementComponent|SetMaxWalkSpeed (Variables|Character|GetCharacterMovement) 0.0)
    (Components|Animation|PlayAnimation (Variables|Character|GetMesh) "/Game/Creatures/PolyArtBoar/Animations/Common/Boar_C_Death1.Boar_C_Death1" false)
    (Utilities|FlowControl|Delay 3.0)
    (Actor|DestroyActor)
    (else
      (Variables|Default|SetFlinch true)
      (Variables|/Script/Engine.CharacterMovementComponent|SetMaxWalkSpeed (Variables|Character|GetCharacterMovement) 5e+02)
      (Utilities|Time|SetTimerbyFunctionName 0 "Reset Walk Speed" 15.0)
      (Pawn|Components|CharacterMovement|DisableMovement (Variables|Character|GetCharacterMovement)))))

(event EventBeginPlay
  (EventDispatchers|AssignOnTakeAnyDamage (delegate Custom|OnTakeAnyDamage_Event_0))
  (bind _outactors (Actor|GetAllActorsOfClass "/Script/NavigationSystem.NavigationData"))
  (for _array_element _outactors
    (Variables|Default|SetNav%20Mesh _array_element))
  (CallFunction|WanderEvent))

(event Collision|EventActorBeginOverlap
  (params (OtherActor :type Actor%20Object%20Reference)))

(fn ConstructionScript
  (bind _bodies (Variables|Default|GetBodies))
  (bind _furs (Variables|Default|GetFurs))
  (bind _tusks (Variables|Default|GetTusks))
  (Class|SkinnedMeshComponent|SetSkeletalMesh (Variables|Character|GetMesh) (Utilities|Array|Get(acopy) _bodies (Math|Random|RandomInteger (Utilities|Array|Length _bodies))) true)
  (Rendering|Material|SetMaterial (Variables|Character|GetMesh) 0 (Utilities|Array|Get(acopy) _furs (Math|Random|RandomInteger (Utilities|Array|Length _furs))))
  (Components|StaticMesh|SetStaticMesh (Variables|Default|GetTusk) (Utilities|Array|Get(acopy) _tusks (Math|Random|RandomInteger (Utilities|Array|Length _tusks)))))

(fn ResetWalkSpeed
  (Variables|/Script/Engine.CharacterMovementComponent|SetMaxWalkSpeed (Variables|Character|GetCharacterMovement) 1e+02))