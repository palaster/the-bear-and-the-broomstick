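; AI controller for NPCs and enemies that sets up the shared NPC blackboard and picks a behavior tree by pawn type.
; On BeginPlay it stores the pawn's spawn point as HomeLocation, then runs the enemy tree, seeding AttackCooldown from BP_Enemy, or the NPC tree otherwise.
; For enemy pawns without a target, perception updates set the Enemy key to any updated BP_Player actor.
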(event OnPerceptionUpdated(AIPerception)
  (params (UpdatedActors :type Array%20of%20Actor%20Object%20References))
  (if (and (Utilities|ClassIsChildOf (Utilities|GetClass (Pawn|GetControlledPawn)) "/Game/Entities/Creatures/BP_Enemy.BP_Enemy_C") (not (Utilities|IsValid (AI|Components|Blackboard|GetValueasObject (AI|GetBlackboard 0) (Utilities|Name|MakeLiteralName "Enemy")))))
    (bind _array_element (Utilities|Array|ForEachLoopwithBreak UpdatedActors :!label _label)
      (:LoopBody
        (if (== (Utilities|GetClass _array_element) "/Game/Player/BP_Player.BP_Player_C")
          (AI|Components|Blackboard|SetValueasObject (AI|GetBlackboard 0) (Utilities|Name|MakeLiteralName "Enemy") _array_element)
          (goto _label Break))))))

(event EventBeginPlay
  (bind _blackboardcomponent (Class|AIController|UseBlackboard "/Game/Entities/Creatures/AI/NPCBlackboard.NPCBlackboard"))
  (AI|Components|Blackboard|SetValueasVector _blackboardcomponent (Utilities|Name|MakeLiteralName "HomeLocation") (Transformation|GetActorLocation (Pawn|GetControlledPawn)))
  (bind _asbp_enemy (Utilities|Casting|CastToBP_Enemy (Pawn|GetControlledPawn))
    (:then
      (AI|Components|Blackboard|SetValueasFloat _blackboardcomponent (Utilities|Name|MakeLiteralName "AttackCooldown") (Variables|/Game/Entities/Creatures/BP_Enemy.BP_Enemy_C|GetAttackCooldown _asbp_enemy))
      (AI|RunBehaviorTree "/Game/Entities/Creatures/AI/EnemyBehaviorTree.EnemyBehaviorTree"))
    (:CastFailed
      (AI|RunBehaviorTree "/Game/Entities/Creatures/AI/NPCBehaviorTree.NPCBehaviorTree"))))

(fn ConstructionScript)