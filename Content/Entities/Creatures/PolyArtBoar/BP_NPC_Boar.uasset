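; BP_NPC_Boar is a boar creature NPC that configures variables and appearance on top of its parent Blueprint's logic.
; Its construction script assigns directional flinch and death montage sets and sets walk and run speeds, then calls the parent construction script.
; It randomizes each boar's look by picking a body mesh, fur material and tusk mesh from arrays.
; The event graph adds no behavior beyond calling the parent's BeginPlay.
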(event EventBeginPlay
  (|CallParentFunction))

(event Collision|EventActorBeginOverlap
  (params (OtherActor :type Actor%20Object%20Reference)))

(event EventTick
  (params (DeltaSeconds :type Float%20%28single-precision%29))
  (|CallParentFunction DeltaSeconds) ; This node is disabled and will not be called.\nDrag off pins to build functionality.
)

(fn ConstructionScript
  (bind _bodies (Variables|Default|GetBodies))
  (bind _furs (Variables|Default|GetFurs))
  (bind _tusks (Variables|Default|GetTusks))
  (Variables|Default|SetFlinchAnims (Utilities|Array|MakeArray "/Game/Entities/Creatures/PolyArtBoar/Animations/Root_Motion/Boar_RM_Damage_Back_Left_Montage.Boar_RM_Damage_Back_Left_Montage" "/Game/Entities/Creatures/PolyArtBoar/Animations/Root_Motion/Boar_RM_Damage_Back_Right_Montage.Boar_RM_Damage_Back_Right_Montage" "/Game/Entities/Creatures/PolyArtBoar/Animations/Root_Motion/Boar_RM_Damage_Left_Montage.Boar_RM_Damage_Left_Montage" "/Game/Entities/Creatures/PolyArtBoar/Animations/Root_Motion/Boar_RM_Damage_Right_Montage.Boar_RM_Damage_Right_Montage"))
  (Variables|Default|SetDeathAnims (Utilities|Array|MakeArray "/Game/Entities/Creatures/PolyArtBoar/Animations/Common/Boar_C_Death1_Montage.Boar_C_Death1_Montage" "/Game/Entities/Creatures/PolyArtBoar/Animations/Common/Boar_C_Death1_Opp_Montage.Boar_C_Death1_Opp_Montage" "/Game/Entities/Creatures/PolyArtBoar/Animations/Common/Boar_C_Death2_Montage.Boar_C_Death2_Montage" "/Game/Entities/Creatures/PolyArtBoar/Animations/Common/Boar_C_Death2_Opp_Montage.Boar_C_Death2_Opp_Montage"))
  (Class|SkinnedMeshComponent|SetSkeletalMesh (Variables|Character|GetMesh) (Utilities|Array|Get(acopy) _bodies (Math|Random|RandomInteger (Utilities|Array|Length _bodies))) true)
  (Rendering|Material|SetMaterial (Variables|Character|GetMesh) 0 (Utilities|Array|Get(acopy) _furs (Math|Random|RandomInteger (Utilities|Array|Length _furs))))
  (Components|StaticMesh|SetStaticMesh (Variables|Default|GetTusk) (Utilities|Array|Get(acopy) _tusks (Math|Random|RandomInteger (Utilities|Array|Length _tusks))))
  (Variables|Default|SetRun%20Speed 5e+02)
  (Variables|Default|SetWalk%20Speed 1.5e+02)
  (|CallParentFunction))