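; Flying enemy creature Blueprint that configures a parent enemy class with its animations and tuning.
; The construction script fills death, attack and aggro montage lists, sets a long fireball attack range and walk and run speeds, then calls the parent script.
; The aggro list reuses a death montage.
; The event graph holds only disabled stubs, so the Blueprint adds no runtime logic.
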(event EventBeginPlay
  (|CallParentFunction) ; This node is disabled and will not be called.\nDrag off pins to build functionality.
)

(event Collision|EventActorBeginOverlap
  (params (OtherActor :type Actor%20Object%20Reference)))

(event EventTick
  (params (DeltaSeconds :type Float%20%28single-precision%29))
  (|CallParentFunction DeltaSeconds) ; This node is disabled and will not be called.\nDrag off pins to build functionality.
)

(fn ConstructionScript
  (Variables|Default|SetDeathAnims (Utilities|Array|MakeArray "/Game/Player/DragonAssets/Animations/Montages/Death/WD_C_Death01_Montage.WD_C_Death01_Montage" "/Game/Player/DragonAssets/Animations/Montages/Death/WD_C_Death01_Opp_Montage.WD_C_Death01_Opp_Montage" "/Game/Player/DragonAssets/Animations/Montages/Death/WD_C_Death02_Montage.WD_C_Death02_Montage" "/Game/Player/DragonAssets/Animations/Montages/Death/WD_C_Death02_Opp_Montage.WD_C_Death02_Opp_Montage"))
  (Variables|Default|SetAttackAnims (Utilities|Array|MakeArray "/Game/Player/DragonAssets/Animations/Montages/WD_C_Attack_FireBall_Montage.WD_C_Attack_FireBall_Montage"))
  (Variables|Default|SetAggroAnims (Utilities|Array|MakeArray "/Game/Player/DragonAssets/Animations/Montages/Death/WD_C_Death01_Montage.WD_C_Death01_Montage"))
  (Variables|Default|SetAttack%20Range 3e+03)
  (Variables|Default|SetWalk%20Speed 1e+02)
  (Variables|Default|SetRun%20Speed 4e+02)
  (|CallParentFunction))