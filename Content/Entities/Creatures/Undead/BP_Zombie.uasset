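; Zombie enemy creature that configures a parent creature Blueprint, which supplies the runtime behavior.
; The construction script fills taunt, death and sword attack montage arrays, sets movement, health and attack stats, and attaches the weapon to the right-hand socket.
; Tick only calls the parent.
; Logic to play a roll montage when the enemy player attacks is disconnected and never runs.
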(event EventBeginPlay
  (|CallParentFunction) ; This node is disabled and will not be called.\nDrag off pins to build functionality.
)

(event Collision|EventActorBeginOverlap
  (params (OtherActor :type Actor%20Object%20Reference)))

(event EventTick
  (params (DeltaSeconds :type Float%20%28single-precision%29))
  (|CallParentFunction DeltaSeconds))

(fn ConstructionScript
  (Variables|Default|SetAggroAnims (Utilities|Array|MakeArray "/Game/Player/HumanAssets/Animations/Taunts/Warrior_Sword_Taunt_A_Anim_Montage.Warrior_Sword_Taunt_A_Anim_Montage" "/Game/Player/HumanAssets/Animations/Taunts/Warrior_Sword_Taunt_B_Anim_Montage.Warrior_Sword_Taunt_B_Anim_Montage" "/Game/Player/HumanAssets/Animations/Taunts/Warrior_Sword_Taunt_C_Anim_Montage.Warrior_Sword_Taunt_C_Anim_Montage"))
  (Variables|Default|SetDeathAnims (Utilities|Array|MakeArray "/Game/Player/HumanAssets/Animations/Deaths/Deaths_Hit_Dazed_Montage.Deaths_Hit_Dazed_Montage" "/Game/Player/HumanAssets/Animations/Deaths/Deaths_Hit_Head_Spinning_Montage.Deaths_Hit_Head_Spinning_Montage" "/Game/Player/HumanAssets/Animations/Deaths/Deaths_Hit_Left_Slow_Bleedout_Montage.Deaths_Hit_Left_Slow_Bleedout_Montage" "/Game/Player/HumanAssets/Animations/Deaths/Deaths_Hit_Mid_Right_Montage.Deaths_Hit_Mid_Right_Montage"))
  (Variables|Default|SetAttackAnims (Utilities|Array|MakeArray "/Game/Player/HumanAssets/Animations/SwordAnims/Warrior_Sword_Attack_13_Anim_Montage.Warrior_Sword_Attack_13_Anim_Montage" "/Game/Player/HumanAssets/Animations/SwordAnims/Warrior_Sword_Attack_14_Anim_Montage.Warrior_Sword_Attack_14_Anim_Montage" "/Game/Player/HumanAssets/Animations/SwordAnims/Warrior_Sword_Attack_15_Anim_Montage.Warrior_Sword_Attack_15_Anim_Montage" "/Game/Player/HumanAssets/Animations/SwordAnims/Warrior_Sword_Attack_16_Anim_Montage.Warrior_Sword_Attack_16_Anim_Montage" "/Game/Player/HumanAssets/Animations/SwordAnims/Warrior_Sword_Attack_17_Anim_Montage.Warrior_Sword_Attack_17_Anim_Montage"))
  (Variables|Default|SetWalk%20Speed 1.5e+02)
  (Variables|Default|SetRun%20Speed 7.5e+02)
  (Variables|Default|SetHP 1.5e+02)
  (Variables|Default|SetAttack%20Speed 1.0)
  (Variables|Default|SetAttack%20Range 5e+01)
  (Variables|Default|SetAttack%20Windup 0.1)
  (Transformation|AttachComponentToComponent (Variables|Default|GetWeapon) (Variables|Character|GetMesh) "hand_r" "KeepRelative" "KeepRelative" "KeepRelative" true)
  (|CallParentFunction))