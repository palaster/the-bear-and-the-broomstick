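; Forest golem enemy Blueprint that configures an inherited creature base as a trunk-swinging melee attacker.
; The construction script fills the death, attack, aggro and flinch montage arrays and sets movement speeds, health, attack speed and range.
; It then attaches the Weapon component to the mesh's Prop1 socket and calls the parent construction script.
; The event graph holds only disabled or empty stubs, with no behavior of its own.
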(event EventBeginPlay
  (|CallParentFunction) ; This node is disabled and will not be called.\nDrag off pins to build functionality.
)

(event Collision|EventActorBeginOverlap
  (params (OtherActor :type Actor%20Object%20Reference)))

(event EventTick
  (params (DeltaSeconds :type Float%20%28single-precision%29)))

(fn ConstructionScript
  (Variables|Default|SetDeathAnims (Utilities|Array|MakeArray "/Game/Entities/Creatures/ForestGolems/Animations/Montages/G_C_Die1_Montage.G_C_Die1_Montage" "/Game/Entities/Creatures/ForestGolems/Animations/Montages/G_C_Die2_Montage.G_C_Die2_Montage" "/Game/Entities/Creatures/ForestGolems/Animations/Montages/G_C_Die3_Montage.G_C_Die3_Montage" "/Game/Entities/Creatures/ForestGolems/Animations/Montages/G_C_Die4_Montage.G_C_Die4_Montage"))
  (Variables|Default|SetAttackAnims (Utilities|Array|MakeArray "/Game/Entities/Creatures/ForestGolems/Animations/Montages/G_C_Trunk_Attack2_Montage.G_C_Trunk_Attack2_Montage" "/Game/Entities/Creatures/ForestGolems/Animations/Montages/G_C_Trunk_Attack3_Montage.G_C_Trunk_Attack3_Montage" "/Game/Entities/Creatures/ForestGolems/Animations/Montages/G_RM_Trunk_Attack_Swing_360_Montage.G_RM_Trunk_Attack_Swing_360_Montage" "/Game/Entities/Creatures/ForestGolems/Animations/Montages/G_RM_Trunk_Attack4_Montage.G_RM_Trunk_Attack4_Montage"))
  (Variables|Default|SetAggroAnims (Utilities|Array|MakeArray "/Game/Entities/Creatures/ForestGolems/Animations/Montages/G_C_Roar_Montage.G_C_Roar_Montage"))
  (Variables|Default|SetFlinchAnims (Utilities|Array|MakeArray "/Game/Entities/Creatures/ForestGolems/Animations/Montages/G_C_Hit_Back_Montage.G_C_Hit_Back_Montage" "/Game/Entities/Creatures/ForestGolems/Animations/Montages/G_C_Hit_Front_Montage.G_C_Hit_Front_Montage" "/Game/Entities/Creatures/ForestGolems/Animations/Montages/G_C_Hit_Left_Montage.G_C_Hit_Left_Montage" "/Game/Entities/Creatures/ForestGolems/Animations/Montages/G_C_Hit_Right_Montage.G_C_Hit_Right_Montage"))
  (Variables|Default|SetWalk%20Speed 135.0)
  (Variables|Default|SetRun%20Speed 4.6e+02)
  (Variables|Default|SetHP 2e+02)
  (Variables|Default|SetAttack%20Speed 1.75)
  (Variables|Default|SetAttack%20Range 2e+02)
  (Transformation|AttachComponentToComponent (Variables|Default|GetWeapon) (Variables|Character|GetMesh) "Prop1" "KeepRelative" "KeepRelative" "KeepRelative" true)
  (|CallParentFunction))