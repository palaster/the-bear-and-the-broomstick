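; BP_NPC is a creature character that alternates between idling and wandering the navmesh, takes damage and dies.
; UpdateAIState dispatches an enum state machine to Idle, Wander, Flinch and Death events, with Tick timing random idle periods before each AI move to a random reachable point.
; Damage stops movement and flashes a red material; death disables key collision responses, plays a random montage with brief global slow motion, then destroys the actor.
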(event Custom|Death_Event
  ;[1 1 1] Death
  (if (not (Variables|Default|GetDead))
    (Variables|Default|SetDead true)
    (Class|NavMovementComponent|StopActiveMovement (Variables|Character|GetCharacterMovement))
    (Collision|SetCollisionResponsetoChannel (Variables|Collision|GetCapsuleComponent) "ECC_Pawn" "ECR_Ignore")
    (Collision|SetCollisionResponsetoChannel (Variables|Collision|GetCapsuleComponent) "ECC_GameTraceChannel4" "ECR_Ignore")
    (Collision|SetCollisionResponsetoChannel (Variables|Collision|GetCapsuleComponent) "ECC_GameTraceChannel1" "ECR_Ignore")
    (Animation|StopAnimMontage 0)
    (Animation|Montage|PlayMontage (Variables|Character|GetMesh) (CallFunction|RandomAnim (Variables|Default|GetDeathAnims))
      (:then
        (Utilities|Time|SetGlobalTimeDilation 0.2)
        (Utilities|FlowControl|Delay 0.25)
        (Utilities|Time|SetGlobalTimeDilation 1.0))
      (:OnCompleted
        (Actor|DestroyActor)))))

(event Custom|OnTakeAnyDamage_Event_0
  (params (DamagedActor :type Actor%20Object%20Reference) (Damage :type Float%20%28single-precision%29) (DamageType :type Damage%20Type%20Object%20Reference) (InstigatedBy :type Controller%20Object%20Reference) (DamageCauser :type Actor%20Object%20Reference))
  ;[1 1 1] Take damage
  (Variables|Default|SetHP (- (Variables|Default|GetHP) Damage))
  (if (not (Variables|Default|GetDead))
    (Components|Movement|StopMovementImmediately (Variables|Character|GetCharacterMovement))
    (if (<= (Variables|Default|GetHP) 0.0)
      (CallFunction|UpdateAIState "NewEnumerator6")
      (else
        (Rendering|Material|SetMaterial (Variables|Character|GetMesh) 0 "/Game/Environment/Materials/red.red")
        (Utilities|FlowControl|Delay 0.1)
        (Rendering|Material|SetMaterial (Variables|Character|GetMesh) 0 (Variables|Default|GetBaseMaterial))))))

(event Custom|Wander_Event
  ;[1 1 1] Wander
  (bind _movementresult (AI|AIMoveTo (Variables|Default|GetNav%20Mesh) self (.RandomLocation (AI|Navigation|GetRandomReachablePointinRadius (Transformation|GetActorLocation) 1e+03 (Variables|Default|GetNav%20Mesh) 0)) 0 5e+01 true)
    (:OnSuccess
      (CallFunction|UpdateAIState "NewEnumerator0"))
    (:OnFail
      (if (not (Utilities|Enum|Equal(Enum) _movementresult "Aborted"))
        (CallFunction|UpdateAIState "NewEnumerator1")))))

(event Custom|Idle_Event
  ;[1 1 1] Set time to idle
  (Variables|Default|SetTimeIdled 0.0)
  (Variables|Default|SetIdleTime (Math|Conversions|ToFloat(Integer) (* (Math|Random|RandomInteger 3) 2)))
  (Components|Movement|StopMovementImmediately (Variables|Character|GetCharacterMovement)))

(event Custom|Flinch_Event
  ;[1 1 1] Flinch
  (Components|Movement|StopMovementImmediately (Variables|Character|GetCharacterMovement))
  (Animation|Montage|PlayMontage (Variables|Character|GetMesh) 0
    (:OnCompleted
      (CallFunction|UpdateAIState "NewEnumerator0"))))

(event EventBeginPlay
  ;[1 1 1] Begin play
  (EventDispatchers|AssignOnTakeAnyDamage (delegate Custom|OnTakeAnyDamage_Event_0))
  (bind _outactors (Actor|GetAllActorsOfClass "/Script/NavigationSystem.NavigationData"))
  (for _array_element _outactors
    (Variables|Default|SetNav%20Mesh _array_element))
  (CallFunction|UpdateAIState "NewEnumerator0"))

(event EventTick
  (params (DeltaSeconds :type Float%20%28single-precision%29))
  ;[1 1 1] Update idle timer
  (if (|Idling)
    (bind _output_get (Variables|Default|SetTimeIdled (|Tick DeltaSeconds)))
    (if (|CanIdle _output_get)
      (CallFunction|UpdateAIState "NewEnumerator1"))))

(fn ConstructionScript
  (CallFunction|ResetWalkSpeed)
  (Variables|Default|SetBaseMaterial (Rendering|Material|GetMaterial (Variables|Character|GetMesh) 0)))

(fn ResetWalkSpeed
  (Variables|/Script/Engine.CharacterMovementComponent|SetMaxWalkSpeed (Variables|Character|GetCharacterMovement) (Variables|Default|GetWalk%20Speed)))

(fn UpdateAIState
  (params (NewParam :type AI_Combat_State%20Enum :default "NewEnumerator0"))
  (bind _output_get (Variables|Default|SetAI%20State NewParam))
  (if (not (Variables|Default|GetDead))
    (switch Utilities|FlowControl|Switch|SwitchonAI_Combat_State _output_get
      (:NewEnumerator0
        (CallFunction|IdleEvent))
      (:NewEnumerator1
        (CallFunction|ResetWalkSpeed)
        (CallFunction|WanderEvent))
      (:NewEnumerator5
        (Pawn|Components|CharacterMovement|DisableMovement (Variables|Character|GetCharacterMovement))
        (Default|CallFlinch))
      (:NewEnumerator6
        (CallFunction|DeathEvent)))))

(fn Unflinch
  (Pawn|Components|CharacterMovement|SetMovementMode (Variables|Character|GetCharacterMovement) "MOVE_Walking" 0)
  (CallFunction|UpdateAIState "NewEnumerator3"))

(fn RandomAnim
  (params (Array :type Array%20of%20Anim%20Montage%20Object%20References))
  (return (Utilities|Array|Get(acopy) Array (Math|Random|RandomInteger (Utilities|Array|Length Array)))))

(fn AnimMoveSpeed
  (return (/ (Math|Vector|VectorLength (Transformation|GetVelocity)) (Variables|Default|GetWalk%20Speed))))