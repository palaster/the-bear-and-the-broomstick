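; Space skybox actor that renders a deep-space backdrop and a stars mesh in a stylized sky.
; The construction script creates dynamic materials for both, sets the space color, and swaps the stars mesh between three layouts by StarModel.
; Each of three star material groups gets its own color and an intensity scaled by overall brightness.
; On Tick, it optionally moves to the player pawn's location.
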(event EventTick
  (params (DeltaSeconds :type Float%20%28single-precision%29))
  (if (Variables|Default|GetShouldFollowPlayer?)
    (Transformation|SetActorLocation (Transformation|GetActorLocation (Game|Player|GetPlayerPawn 0)) false false)))

(fn ConstructionScript
  ;[1 1 1] Create material instances for modification
  (bind _returnvalue (Rendering|Material|CreateDynamicMaterialInstance (Variables|Default|GetDeepSpace) 0 "/Game/Environment/StylizedSky/Materials/Sky/SpaceBox_Mat.SpaceBox_Mat" "None" :!class /Script/Engine.PrimitiveComponent))
  (Variables|Space|SetDeepSpaceMatInst _returnvalue)
  (bind _returnvalue_2 (Rendering|Material|CreateDynamicMaterialInstance (Variables|Default|GetStarsMesh) 0 "/Game/Environment/StylizedSky/Materials/Sky/Stars01_Mat.Stars01_Mat" "None" :!class /Script/Engine.PrimitiveComponent))
  (Variables|Stars|SetStarsColor01MatInst _returnvalue_2)
  (bind _returnvalue_3 (Rendering|Material|CreateDynamicMaterialInstance (Variables|Default|GetStarsMesh) 1 "/Game/Environment/StylizedSky/Materials/Sky/Stars02_Mat.Stars02_Mat" "None" :!class /Script/Engine.PrimitiveComponent))
  (Variables|Stars|SetStarsColor02MatInst _returnvalue_3)
  (bind _returnvalue_4 (Rendering|Material|CreateDynamicMaterialInstance (Variables|Default|GetStarsMesh) 2 "/Game/Environment/StylizedSky/Materials/Sky/Stars03_Mat.Stars03_Mat" "None" :!class /Script/Engine.PrimitiveComponent))
  (Variables|Stars|SetStarsColor03MatInst _returnvalue_4)
  ;[1 1 1] Set Space color
  (Rendering|Material|SetVectorParameterValue (Variables|Space|GetDeepSpaceMatInst) "SpaceColor" (Variables|Space|GetSpaceColor) :!class /Script/Engine.MaterialInstanceDynamic)
  ;[1 1 1] Set mesh selection
  (Components|StaticMesh|SetStaticMesh (Variables|Default|GetStarsMesh) (Utilities|Select :Index (Variables|Stars|GetStar%20Model) :NewEnumerator0 "/Game/Environment/StylizedSky/Meshes/Sky/Sky_Stars_Galaxy_01_SM.Sky_Stars_Galaxy_01_SM" :NewEnumerator1 "/Game/Environment/StylizedSky/Meshes/Sky/Sky_Stars_Scrambled_02_SM.Sky_Stars_Scrambled_02_SM" :NewEnumerator2 "/Game/Environment/StylizedSky/Meshes/Sky/Sky_Stars_AllOverThePlace_03_SM.Sky_Stars_AllOverThePlace_03_SM"))
  ;[1 1 1] Set custom colors
  (for (_array_element _array_index) (Utilities|Array|MakeArray (Variables|Stars|GetStarsColor01MatInst) (Variables|Stars|GetStarsColor02MatInst) (Variables|Stars|GetStarsColor03MatInst))
    (Rendering|Material|SetScalarParameterValue _array_element "Brightness" (* (.intensity (Utilities|Select :Index _array_index :Option%200 (Variables|Stars|GetStarGroup01) :Option%201 (Variables|Stars|GetStarGroup02) :Option%202 (Variables|Stars|GetStarGroup03))) (Variables|Stars|GetOverallStarBrightness)) :!class /Script/Engine.MaterialInstanceDynamic) ; Set brightness multiplier insidestar material
    (Rendering|Material|SetVectorParameterValue _array_element "StarColor" (.color (Utilities|Select :Index _array_index :Option%200 (Variables|Stars|GetStarGroup01) :Option%201 (Variables|Stars|GetStarGroup02) :Option%202 (Variables|Stars|GetStarGroup03))) :!class /Script/Engine.MaterialInstanceDynamic) ; Set color inside star material
  ))