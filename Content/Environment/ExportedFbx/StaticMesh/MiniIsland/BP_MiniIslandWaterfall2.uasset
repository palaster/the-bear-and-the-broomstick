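; Mini-island water actor that drives a stylized lake material on its CartoonWater component.
; Construction creates a dynamic instance of the lake material selected by OceanType (lit, unlit, transparency, tessellation, mobile variants).
; WaterParameters, rerun at BeginPlay, pushes look settings to that instance and wave, tessellation and water level to the shared MPC_Lake collection.
; A looping timer optionally refreshes Ocean Level from mesh height; texture overrides are unconnected.
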(event EventBeginPlay
  (CallFunction|WaterParameters)
  (Utilities|Time|SetTimerbyFunctionName 0 "Update Water" 0.1 true))

(fn ConstructionScript
  (Utilities|FlowControl|Sequence
    (:then_0
      (bind _returnvalue (Rendering|Material|CreateDynamicMaterialInstance (Variables|Default|GetCartoonWater) 0 (Utilities|Select :Index (Variables|GlobalParameters|GetOcean%20Type) :NewEnumerator53 "/Game/Environment/Water/Materials/Water/Lake/MI_Lake_UNLIT_Transparent_Tessellated.MI_Lake_UNLIT_Transparent_Tessellated" :NewEnumerator55 "/Game/Environment/Water/Materials/Water/Lake/MI_Lake_UNLIT_Transparent_NonTessellated.MI_Lake_UNLIT_Transparent_NonTessellated" :NewEnumerator54 "/Game/Environment/Water/Materials/Water/Lake/MI_Lake_UNLIT_NonTransparent_Tessellated.MI_Lake_UNLIT_NonTransparent_Tessellated" :NewEnumerator56 "/Game/Environment/Water/Materials/Water/Lake/MI_Lake_UNLIT_NonTransparent_NonTessellated.MI_Lake_UNLIT_NonTransparent_NonTessellated" :NewEnumerator57 0 :NewEnumerator58 "/Game/Environment/Water/Materials/Water/Lake/MI_Lake_PBR_Transparent_Tessellated.MI_Lake_PBR_Transparent_Tessellated" :NewEnumerator60 "/Game/Environment/Water/Materials/Water/Lake/MI_Lake_PBR_Transparent_NonTessellated.MI_Lake_PBR_Transparent_NonTessellated" :NewEnumerator59 "/Game/Environment/Water/Materials/Water/Lake/MI_Lake_PBR_NonTransparent_Tessellated.MI_Lake_PBR_NonTransparent_Tessellated" :NewEnumerator61 "/Game/Environment/Water/Materials/Water/Lake/MI_Lake_PBR_NonTransparent_NonTessellated.MI_Lake_PBR_NonTransparent_NonTessellated" :NewEnumerator62 0 :NewEnumerator63 "/Game/Environment/Water/Materials/Water/Lake/MI_Lake_Mobile_Transparent.MI_Lake_Mobile_Transparent" :NewEnumerator64 "/Game/Environment/Water/Materials/Water/Lake/MI_Lake_Mobile_NonTransparent.MI_Lake_Mobile_NonTransparent" :NewEnumerator65 0 :NewEnumerator66 0) "None" :!class /Script/Engine.PrimitiveComponent))
      (bind _output_get (Variables|Default|SetCurrent%20Material%20 _returnvalue))
      (Rendering|Material|SetMaterial (Variables|Default|GetCartoonWater) 0 _output_get))
    (:then_1
      (CallFunction|WaterParameters))))

(fn WaterParameters
  (bind _current_material_ (Variables|Default|GetCurrent%20Material%20))
  (bind _current_material__2 (Variables|Default|GetCurrent%20Material%20))
  (bind _current_material__3 (Variables|Default|GetCurrent%20Material%20))
  (bind _current_material__4 (Variables|Default|GetCurrent%20Material%20))
  (bind _current_material__5 (Variables|Default|GetCurrent%20Material%20))
  (bind _current_material__6 (Variables|Default|GetCurrent%20Material%20))
  (bind _current_material__7 (Variables|Default|GetCurrent%20Material%20))
  (bind _current_material__8 (Variables|Default|GetCurrent%20Material%20))
  (bind _current_material__9 (Variables|Default|GetCurrent%20Material%20))
  (bind _current_material__10 (Variables|Default|GetCurrent%20Material%20))
  (bind _current_material__11 (Variables|Default|GetCurrent%20Material%20))
  (Utilities|FlowControl|Sequence
    (:then_0
      ;[1 1 1] Global Parameters
      (Rendering|Material|SetScalarParameterValue "/Game/Environment/Water/Materials/MaterialCollections/MPC_Lake.MPC_Lake" "Wave Speed Global" (Variables|GlobalParameters|GetWave%20Speed) :!class /Script/Engine.KismetMaterialLibrary)
      (Rendering|Material|SetScalarParameterValue _current_material__7 "Global Opacity" (Variables|GlobalParameters|GetGlobal%20Opacity) :!class /Script/Engine.MaterialInstanceDynamic)
      (Rendering|Material|SetScalarParameterValue "/Game/Environment/Water/Materials/MaterialCollections/MPC_Lake.MPC_Lake" "Day Intensity" (Variables|GlobalParameters|GetDay%20Intensity) :!class /Script/Engine.KismetMaterialLibrary)
      (Rendering|Material|SetScalarParameterValue _current_material__7 "Water Depth" (Variables|GlobalParameters|GetWater%20Depth) :!class /Script/Engine.MaterialInstanceDynamic)
      (Rendering|Material|SetScalarParameterValue _current_material__7 "Sun Reflection Intensity" (Variables|GlobalParameters|GetSun%20Reflection%20Intensity) :!class /Script/Engine.MaterialInstanceDynamic)
      (Rendering|Material|SetScalarParameterValue _current_material__7 "Sun Reflection Tightness" (Variables|GlobalParameters|GetSun%20Reflection%20Tightness) :!class /Script/Engine.MaterialInstanceDynamic)
      (Rendering|Material|SetScalarParameterValue _current_material__7 "Shore Distance" (Variables|GlobalParameters|GetShore%20Distance) :!class /Script/Engine.MaterialInstanceDynamic)
      (Rendering|Material|SetScalarParameterValue "/Game/Environment/Water/Materials/MaterialCollections/MPC_Lake.MPC_Lake" "Tesselation Factor" (Variables|GlobalParameters|GetTessellation%20Factor) :!class /Script/Engine.KismetMaterialLibrary))
    (:then_1
      ;[1 1 1] Gerstner Waves
      (Rendering|Material|SetScalarParameterValue "/Game/Environment/Water/Materials/MaterialCollections/MPC_Lake.MPC_Lake" "Wave Length" (Variables|GerstnerWave|GetWave%20Length) :!class /Script/Engine.KismetMaterialLibrary)
      (Rendering|Material|SetScalarParameterValue "/Game/Environment/Water/Materials/MaterialCollections/MPC_Lake.MPC_Lake" "Amplitude" (Variables|GerstnerWave|GetAmplitude) :!class /Script/Engine.KismetMaterialLibrary)
      (Rendering|Material|SetScalarParameterValue "/Game/Environment/Water/Materials/MaterialCollections/MPC_Lake.MPC_Lake" "Steepness" (Variables|GerstnerWave|GetSteepness) :!class /Script/Engine.KismetMaterialLibrary)
      (Rendering|Material|SetScalarParameterValue "/Game/Environment/Water/Materials/MaterialCollections/MPC_Lake.MPC_Lake" "Gerstner Wave Speed " (Variables|GerstnerWave|GetGerstner%20Wave%20Speed%20) :!class /Script/Engine.KismetMaterialLibrary)
      (Rendering|Material|SetScalarParameterValue "/Game/Environment/Water/Materials/MaterialCollections/MPC_Lake.MPC_Lake" "Wind Direction" (Variables|GerstnerWave|GetWind%20Direction) :!class /Script/Engine.KismetMaterialLibrary))
    (:then_2
      ;[1 1 1] Distances
      (Rendering|Material|SetScalarParameterValue _current_material__11 "Color Distance Fade" (Variables|Distances|GetColor%20Distance%20Fade) :!class /Script/Engine.MaterialInstanceDynamic)
      (Rendering|Material|SetScalarParameterValue _current_material__11 "Color Distance Falloff" (Variables|Distances|GetColor%20Distance%20Falloff) :!class /Script/Engine.MaterialInstanceDynamic)
      (Rendering|Material|SetScalarParameterValue _current_material__11 "Water Depth Distance Fade" (Variables|Distances|GetWater%20Depth%20Distance%20Fade) :!class /Script/Engine.MaterialInstanceDynamic)
      (Rendering|Material|SetScalarParameterValue _current_material__11 "Water Depth Distance Falloff" (Variables|Distances|GetWater%20Depth%20Distance%20Falloff) :!class /Script/Engine.MaterialInstanceDynamic)
      (Rendering|Material|SetScalarParameterValue _current_material__11 "Foam Distance Fade" (Variables|Distances|GetFoam%20Distance%20Fade) :!class /Script/Engine.MaterialInstanceDynamic)
      (Rendering|Material|SetScalarParameterValue _current_material__11 "Foam Distance Falloff" (Variables|Distances|GetFoam%20Distance%20Falloff) :!class /Script/Engine.MaterialInstanceDynamic)
      (Rendering|Material|SetScalarParameterValue _current_material__11 "Normal Distance Fade" (Variables|Distances|GetNormal%20Distance%20Fade) :!class /Script/Engine.MaterialInstanceDynamic)
      (Rendering|Material|SetScalarParameterValue _current_material__11 "Normal Distance Falloff" (Variables|Distances|GetNormal%20Distance%20Falloff) :!class /Script/Engine.MaterialInstanceDynamic)
      (Rendering|Material|SetScalarParameterValue _current_material__11 "Refraction Distance Fade" (Variables|Distances|GetRefraction%20Distance%20Fade) :!class /Script/Engine.MaterialInstanceDynamic)
      (Rendering|Material|SetScalarParameterValue _current_material__11 "Refraction Distance Falloff" (Variables|Distances|GetRefraction%20Distance%20Falloff) :!class /Script/Engine.MaterialInstanceDynamic)
      (Rendering|Material|SetScalarParameterValue _current_material__11 "SSS Distance Fade" (Variables|Distances|GetSSS%20Distance%20Fade) :!class /Script/Engine.MaterialInstanceDynamic)
      (Rendering|Material|SetScalarParameterValue _current_material__11 "SSS Distance Falloff" (Variables|Distances|GetSSS%20Distance%20Falloff) :!class /Script/Engine.MaterialInstanceDynamic))
    (:then_3
      ;[1 1 1] Normals
      (Rendering|Material|SetScalarParameterValue _current_material__10 "Small Normal Speed" (Variables|Normals|GetSmall%20Normal%20Speed) :!class /Script/Engine.MaterialInstanceDynamic)
      (Rendering|Material|SetScalarParameterValue _current_material__10 "Small Normal Intensity" (Variables|Normals|GetSmall%20Normal%20Intensity) :!class /Script/Engine.MaterialInstanceDynamic)
      (Rendering|Material|SetScalarParameterValue _current_material__10 "Small Normal Tiling" (Variables|Normals|GetSmall%20Normal%20Tiling) :!class /Script/Engine.MaterialInstanceDynamic)
      (Rendering|Material|SetScalarParameterValue _current_material__10 "Large Normal Speed" (Variables|Normals|GetLarge%20Normal%20Speed) :!class /Script/Engine.MaterialInstanceDynamic)
      (Rendering|Material|SetScalarParameterValue _current_material__10 "Large Normal Intensity" (Variables|Normals|GetLarge%20Normal%20Intensity) :!class /Script/Engine.MaterialInstanceDynamic)
      (Rendering|Material|SetScalarParameterValue _current_material__10 "Large Normal Tiling" (Variables|Normals|GetLarge%20Normal%20Tiling) :!class /Script/Engine.MaterialInstanceDynamic))
    (:then_4
      ;[1 1 1] Seafoam
      (Rendering|Material|SetScalarParameterValue _current_material__9 "Seafoam Intensity" (Variables|Seafoam|GetSeafoam%20Intensity) :!class /Script/Engine.MaterialInstanceDynamic)
      (Rendering|Material|SetScalarParameterValue _current_material__9 "Seafoam Base Height" (Variables|Seafoam|GetSeafoam%20Base%20Height) :!class /Script/Engine.MaterialInstanceDynamic)
      (Rendering|Material|SetScalarParameterValue _current_material__9 "Seafoam Softness" (Variables|Seafoam|GetSeafoam%20Softness) :!class /Script/Engine.MaterialInstanceDynamic)
      (Rendering|Material|SetScalarParameterValue _current_material__9 "Seafoam Distorsion" (Variables|Seafoam|GetSeafoam%20Distorsion) :!class /Script/Engine.MaterialInstanceDynamic)
      (Rendering|Material|SetScalarParameterValue _current_material__9 "Seafoam Tiling" (Variables|Seafoam|GetSeafoam%20Tiling) :!class /Script/Engine.MaterialInstanceDynamic))
    (:then_5
      ;[1 1 1] Foam
      (Rendering|Material|SetScalarParameterValue _current_material__8 "Foam Intensity" (Variables|Foam|GetFoam%20Intensity) :!class /Script/Engine.MaterialInstanceDynamic)
      (Rendering|Material|SetScalarParameterValue _current_material__8 "Foam Speed" (Variables|Foam|GetFoam%20Speed) :!class /Script/Engine.MaterialInstanceDynamic)
      (Rendering|Material|SetScalarParameterValue _current_material__8 "Foam X Tile" (Variables|Foam|GetFoam%20X%20Tile) :!class /Script/Engine.MaterialInstanceDynamic)
      (Rendering|Material|SetScalarParameterValue _current_material__8 "Foam Y Tile" (Variables|Foam|GetFoam%20Y%20Tile) :!class /Script/Engine.MaterialInstanceDynamic)
      (Rendering|Material|SetScalarParameterValue _current_material__8 "Intersection Size" (Variables|Foam|GetIntersection%20Size) :!class /Script/Engine.MaterialInstanceDynamic)
      (Rendering|Material|SetScalarParameterValue _current_material__8 "Intersection Softness" (Variables|Foam|GetIntersection%20Softness) :!class /Script/Engine.MaterialInstanceDynamic)
      (Rendering|Material|SetScalarParameterValue _current_material__8 "Intersection Size Reduction Over Distance" (Variables|Foam|GetIntersection%20Size%20Reduction%20Over%20Distance) :!class /Script/Engine.MaterialInstanceDynamic))
    (:then_6
      ;[1 1 1] Cubemap
      (Rendering|Material|SetScalarParameterValue _current_material__6 "CubeMap Intensity" (Variables|Reflection|GetCubeMap%20Intensity) :!class /Script/Engine.MaterialInstanceDynamic)
      (Rendering|Material|SetScalarParameterValue _current_material__6 "Reflection Angle" (Variables|Reflection|GetReflection%20Angle) :!class /Script/Engine.MaterialInstanceDynamic)
      (Rendering|Material|SetScalarParameterValue _current_material__6 "Specular Intensity" (Variables|Reflection|GetSpecular%20Intensity) :!class /Script/Engine.MaterialInstanceDynamic))
    (:then_7
      ;[1 1 1] Refraction
      (Rendering|Material|SetScalarParameterValue _current_material__5 "Refraction Amount" (Variables|Refraction|GetRefraction%20Amount) :!class /Script/Engine.MaterialInstanceDynamic)
      (Rendering|Material|SetScalarParameterValue _current_material__5 "Refraction Amount Depth" (Variables|Underwater|GetRefraction%20Amount%20Depth) :!class /Script/Engine.MaterialInstanceDynamic)
      (Rendering|Material|SetScalarParameterValue _current_material__5 "Refraction Depth" (Variables|Underwater|GetRefraction%20Depth) :!class /Script/Engine.MaterialInstanceDynamic))
    (:then_8
      ;[1 1 1] Highlight
      (Rendering|Material|SetScalarParameterValue _current_material__4 "Highlight Intensity" (Variables|Highlight|GetHighlight%20Intensity) :!class /Script/Engine.MaterialInstanceDynamic)
      (Rendering|Material|SetScalarParameterValue _current_material__4 "Highlight Base Height" (Variables|Highlight|GetHighlight%20Base%20Height) :!class /Script/Engine.MaterialInstanceDynamic)
      (Rendering|Material|SetScalarParameterValue _current_material__4 "Highlight Softness" (Variables|Highlight|GetHighlight%20Softness) :!class /Script/Engine.MaterialInstanceDynamic)
      (Rendering|Material|SetScalarParameterValue _current_material__4 "Highlight Density" (Variables|Highlight|GetHighlight%20Density) :!class /Script/Engine.MaterialInstanceDynamic))
    (:then_9
      ;[1 1 1] Trough
      (Rendering|Material|SetScalarParameterValue _current_material__3 "Trough Intensity" (Variables|Trough|GetTrough%20Intensity) :!class /Script/Engine.MaterialInstanceDynamic)
      (Rendering|Material|SetScalarParameterValue _current_material__3 "Trough Base Height" (Variables|Trough|GetTrough%20Base%20Height) :!class /Script/Engine.MaterialInstanceDynamic)
      (Rendering|Material|SetScalarParameterValue _current_material__3 "Trough Softness" (Variables|Trough|GetTrough%20Softnes) :!class /Script/Engine.MaterialInstanceDynamic))
    (:then_10
      ;[1 1 1] SSS
      (Rendering|Material|SetScalarParameterValue _current_material__2 "SSS Intensity" (Variables|SubsurfaceScattering|GetSSS%20Intensity) :!class /Script/Engine.MaterialInstanceDynamic)
      (Rendering|Material|SetScalarParameterValue _current_material__2 "SSS Base Height" (Variables|SubsurfaceScattering|GetSSS%20Base%20Height) :!class /Script/Engine.MaterialInstanceDynamic)
      (Rendering|Material|SetScalarParameterValue _current_material__2 "SSS Softness" (Variables|SubsurfaceScattering|GetSSS%20Softness) :!class /Script/Engine.MaterialInstanceDynamic))
    (:then_11
      ;[1 1 1] Colors
      (Rendering|Material|SetVectorParameterValue _current_material_ "Base Color" (Variables|Colors|GetBase%20Color) :!class /Script/Engine.MaterialInstanceDynamic)
      (Rendering|Material|SetVectorParameterValue _current_material_ "Far Color" (Variables|Colors|GetFar%20Color) :!class /Script/Engine.MaterialInstanceDynamic)
      (Rendering|Material|SetVectorParameterValue _current_material_ "Shallow Water Color" (Variables|Colors|GetShallow%20Water%20Color) :!class /Script/Engine.MaterialInstanceDynamic)
      (Rendering|Material|SetVectorParameterValue _current_material_ "Trough Color" (Variables|Colors|GetTrough%20Color) :!class /Script/Engine.MaterialInstanceDynamic)
      (Rendering|Material|SetVectorParameterValue _current_material_ "SSS Color" (Variables|Colors|GetSSS%20Color) :!class /Script/Engine.MaterialInstanceDynamic)
      (Rendering|Material|SetVectorParameterValue _current_material_ "Foam Color" (Variables|Colors|GetFoam%20Color) :!class /Script/Engine.MaterialInstanceDynamic)
      (Rendering|Material|SetVectorParameterValue _current_material_ "Seafoam Color" (Variables|Colors|GetSeafoam%20Color) :!class /Script/Engine.MaterialInstanceDynamic))
    (:then_12
      ;[1 1 1] Location Z
      (Rendering|Material|SetScalarParameterValue "/Game/Environment/Water/Materials/MaterialCollections/MPC_Lake.MPC_Lake" "Ocean Level" (.z (Transformation|GetWorldLocation (Variables|Default|GetCartoonWater))) :!class /Script/Engine.KismetMaterialLibrary))))

(fn UpdateWater
  (if (Variables|GlobalParameters|GetUpdate%20WaterMesh%20Transform%20Runtime)
    (Rendering|Material|SetScalarParameterValue "/Game/Environment/Water/Materials/MaterialCollections/MPC_Lake.MPC_Lake" "Ocean Level" (.z (Transformation|GetWorldLocation (Variables|Default|GetCartoonWater))) :!class /Script/Engine.KismetMaterialLibrary)))