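; BP_AreaSpawner is a demo-style emitter in the StylizedVFX fire pack that rains fire projectiles from a box volume.
; Each Tick it rolls a one-in-MaxRandom chance to spawn a BP_Projectile at a random point inside its Box, oriented by the Arrow's relative rotation.
; A coin flip picks between a slower charged fireball with a medium explosion and a faster fire ray with a small explosion.
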(event EventBeginPlay)

(event Collision|EventActorBeginOverlap
  (params (OtherActor :type Actor%20Object%20Reference)))

(event EventTick
  (params (DeltaSeconds :type Float%20%28single-precision%29))
  (bind _box (Variables|Default|GetBox))
  (bind _returnvalue (Transformation|GetWorldLocation _box))
  (bind _boxextent (Variables|/Script/Engine.BoxComponent|GetBoxExtent _box))
  (bind _returnvalue_2 (Math|Random|RandomPointinBoundingBox _returnvalue _boxextent))
  (if (== (Math|Random|RandomIntegerinRange 1 (Variables|Default|GetmaxRandom)) 1)
    (if (Math|Random|RandomBool)
      (Game|SpawnActorfromClass "/Game/Particles/StylizedVFX_Fire/Blueprints/BP_Projectile.BP_Projectile_C" (Math|Transform|MakeTransform _returnvalue_2 (Variables|/Script/Engine.SceneComponent|GetRelativeRotation (Variables|Default|GetArrow)) "1,1,1") "AlwaysSpawn" 0 "/Game/Particles/StylizedVFX_Fire/Effects/P_FireBall_Charge.P_FireBall_Charge" 1e+03 1e+03 "/Game/Particles/StylizedVFX_Fire/Effects/P_FireExplosion_Medium.P_FireExplosion_Medium" 0)
      (else
        (Game|SpawnActorfromClass "/Game/Particles/StylizedVFX_Fire/Blueprints/BP_Projectile.BP_Projectile_C" (Math|Transform|MakeTransform _returnvalue_2 (Variables|/Script/Engine.SceneComponent|GetRelativeRotation (Variables|Default|GetArrow)) "1,1,1") "AlwaysSpawn" 0 "/Game/Particles/StylizedVFX_Fire/Effects/P_FireRay.P_FireRay" 3e+03 3e+03 "/Game/Particles/StylizedVFX_Fire/Effects/P_FireExplosion_Small.P_FireExplosion_Small" 0)))))

(fn ConstructionScript)