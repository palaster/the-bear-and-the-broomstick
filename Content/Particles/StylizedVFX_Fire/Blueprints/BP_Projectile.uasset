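; BP_Projectile is a configurable VFX projectile from the StylizedVFX_Fire content that flies with a particle effect and explodes on impact.
; The construction script applies the particle template and speed variables to its particle and projectile movement components.
; The first sphere hit spawns an auto-released pooled explosion emitter at the impact point and shortens the actor's lifespan.
; Every hit also prints a display name.
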(event OnComponentHit(Sphere)
  (params (HitComponent :type Primitive%20Component%20Object%20Reference) (OtherActor :type Actor%20Object%20Reference) (OtherComp :type Primitive%20Component%20Object%20Reference) (NormalImpulse :type Vector :default "0, 0, 0") (Hit :type Hit%20Result%20Structure%20%28by%20ref%29))
  (Development|PrintString (Utilities|GetDisplayName 0))
  (Utilities|FlowControl|DoOnce false
    (:Completed
      (Effects|SpawnEmitteratLocation (Variables|Default|GetExplosionTemplate) (.ImpactPoint (Collision|BreakHitResult Hit)) "0, 0, 0" "1.000000,1.000000,1.000000" true "AutoRelease")
      (Actor|SetLifeSpan 0.2))))

(event EventBeginPlay)

(event Collision|EventActorBeginOverlap
  (params (OtherActor :type Actor%20Object%20Reference)))

(event EventTick
  (params (DeltaSeconds :type Float%20%28single-precision%29)))

(fn ConstructionScript
  (bind _projectilemovement (Variables|Default|GetProjectileMovement))
  (Effects|Components|ParticleSystem|SetTemplate (Variables|Default|GetParticleSystem) (Variables|Default|GetParticleTemplate))
  (Variables|/Script/Engine.ProjectileMovementComponent|SetInitialSpeed _projectilemovement (Variables|Default|GetInitSpeed))
  (Variables|/Script/Engine.ProjectileMovementComponent|SetMaxSpeed _projectilemovement (Variables|Default|GetmaxSpeed)))